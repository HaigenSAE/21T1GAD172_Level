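; BP_LevelEnd_Master is a level-end goal that runs a celebration when the player character enters its EndTrigger volume, then returns to the HUB_Draft level.
; On overlap it snaps the player to the actor's X and Y while keeping their height, then disables input.
; It swaps the idle particle system for a Celebrate effect, plays a celebrate animation and victory sound, and loads the hub after a short delay.
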(event `self.EndTrigger.OnComponentBeginOverlap`
  (params (OverlappedComponent :type "PrimitiveComponent Object Reference") (OtherActor :type "Actor Object Reference") (OtherComp :type "PrimitiveComponent Object Reference") (OtherBodyIndex :type Integer) (bFromSweep :type Boolean) (SweepResult :type "HitResult Structure (by ref)"))
  (bind _returnvalue (`GameplayStatics.GetPlayerCharacter` 0))
  (bind (_returnvalue_x _returnvalue_y) (`KismetMathLibrary.BreakVector` (`self.K2_GetActorLocation`)))
  (bind (_returnvalue_x_2 _returnvalue_y_2 _returnvalue_z) (`KismetMathLibrary.BreakVector` (`self.K2_GetActorLocation` _returnvalue)))
  (if (== OtherActor _returnvalue)
    (`self.K2_SetActorLocation` _returnvalue (`KismetMathLibrary.MakeVector` _returnvalue_x _returnvalue_y _returnvalue_z) false false)
    (`ActorComponent.Deactivate` (`self.ParticleSystem`))
    (`ActorComponent.Activate` (`self.Celebrate`) true)
    (`self.DisableInput` _returnvalue (`GameplayStatics.GetPlayerController` 0))
    (`SkeletalMeshComponent.PlayAnimation` (`Character.Mesh` (cast `/Game/Assets/LearningKit_Games/Blueprints/PlayerCharacter/BP_LearningKit_PlayerCharacter` _returnvalue :!pure true)) "/Game/Assets/LearningKit_Games/Assets/Characters/Character/Animations/EpicCharacter_Celebrate.EpicCharacter_Celebrate" false)
    (`GameplayStatics.PlaySound2D` "/Game/MegaGameMusicCollection/8BitActionGameLoops/Wavs/Victory.Victory" 1.0 1.0 0.0 null null)
    (`KismetSystemLibrary.Delay` 3.0)
    (`GameplayStatics.OpenLevelBySoftObjectPtr` "/Game/Maps/HUB_Draft.HUB_Draft")))

(fn `UserConstructionScript`)